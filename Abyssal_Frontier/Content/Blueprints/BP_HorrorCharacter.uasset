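; Horror player character Blueprint that adds time-based breathing exhaustion and an item inspection mode.
; Tick accumulates elapsed time to raise the Breathing MetaSound's Exhaustion parameter over five minutes, sending the inverse through the sprint meter update event.
; InspectItem shows the item's mesh and stops walking; mouse look rotates it while still aiming, and X exits.
; BeginPlay also resets O2Meter and pushes the master sound mix.
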(event Input|EnhancedActionEvents|EnhancedInputActionIA_MouseLook
  (params (ActionValue :type Vector%202D%20Structure) (ElapsedSeconds :type Float%20%28double-precision%29) (TriggeredSeconds :type Float%20%28double-precision%29) (InputAction :type Input%20Action%20Object%20Reference :default "/Game/Input/Actions/IA_MouseLook.IA_MouseLook"))
  (CallFunction|Aim (.x ActionValue) (.y ActionValue))
  (if (Variables|Default|GetisInspecting?)
    (Transformation|AddLocalRotation (Variables|Default|GetInspect%20Item%20Mesh) (Math|Rotator|MakeRotator (* (.y ActionValue) -1.0) 0.0 (* (.x ActionValue) -1.0)) false false)))

(event EventTick
  (params (DeltaSeconds :type Float%20%28single-precision%29))
  ;[0 0.4165 0.8698 0.5] Set exhaustion input in metasound
  (bind _output_get (Variables|Default|SetTime%20Passed (+ DeltaSeconds (Variables|Default|GetTime%20Passed))))
  (Audio|Parameter|SetFloatParameter (Variables|Default|GetBreathing) "Exhaustion" (/ _output_get 3e+02) :!class /Script/AudioExtensions.AudioParameterControllerInterface)
  (Default|CallOnSprintMeterUpdated (- 1.0 (/ _output_get 3e+02))))

(event EventBeginPlay
  (|CallParentFunction)
  (Variables|Sprint|SetO2%20Meter 0.0)
  (Audio|PushSoundMixModifier "/Game/Audio/SoundClasses/SM_Master.SM_Master"))

(event Input|KeyboardEvents|X
  (params (Key :type Key%20Structure :default "None"))
  (:Pressed
    (if (Variables|Default|GetisInspecting?)
      (Variables|Default|SetisInspecting? false)
      (Rendering|SetVisibility (Variables|Default|GetInspect%20Item%20Mesh) false false)
      (Variables|/Script/Engine.CharacterMovementComponent|SetMaxWalkSpeed (Variables|Character|GetCharacterMovement) (Variables|Default|GetWalk%20Speed)))))

(fn ConstructionScript
  (|CallParentFunction))

(fn InspectItem
  (params (Item%20Structure :type S%20Item%20Structure%20Structure))
  (bind _inspect_item_mesh (Variables|Default|GetInspect%20Item%20Mesh))
  (Variables|Default|SetisInspecting? true)
  (Components|StaticMesh|SetStaticMesh _inspect_item_mesh (.mesh Item%20Structure))
  (Rendering|SetVisibility _inspect_item_mesh true false)
  (Variables|/Script/Engine.CharacterMovementComponent|SetMaxWalkSpeed (Variables|Character|GetCharacterMovement) 0.0))